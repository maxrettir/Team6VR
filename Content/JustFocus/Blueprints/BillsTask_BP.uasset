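; BillsTask_BP is a VR grabbable task object, apparently for bills, that a motion controller can pick up and drop.
; Pickup turns off mesh physics and attaches the root to the given component, keeping world transform; Drop restores physics and detaches.
; Overlapping the Target actor prints a collision message and casts Popup to TestPopup_BP, with nothing following the cast yet.
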(event EventBeginPlay)

(event Collision|EventActorBeginOverlap
  (params (OtherActor :type Actor%20Object%20Reference))
  (if (== OtherActor (Variables|Default|GetTarget))
    (Development|PrintString "Collision")
    (Utilities|Casting|CastToTestPopup_BP (Variables|Default|GetPopup))))

(event EventTick
  (params (DeltaSeconds :type Float%20%28single-precision%29)))

(event EventPickup
  (params (AttachTo :type Scene%20Component%20Object%20Reference))
  (Physics|SetSimulatePhysics (Variables|Debug|GetStaticMeshComponent) false)
  (Transformation|AttachComponentToComponent (VehicleSound|GetRootComponent) AttachTo "None" "KeepWorld" "KeepWorld" "KeepWorld" false))

(event EventDrop
  (Physics|SetSimulatePhysics (Variables|Debug|GetStaticMeshComponent) true)
  (Transformation|DetachFromActor "KeepWorld" "KeepWorld" "KeepWorld"))

(fn ConstructionScript)