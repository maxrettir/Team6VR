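; A task object actor that can be picked up and dropped, and that signals task completion on overlap.
; The first overlap with any actor calls CallTaskFinish and sets IsDone to block repeats; a comparison against Target is left unused.
; Pickup disables mesh physics, attaches the root to the supplied component keeping world transform, and hides the widget.
; Drop detaches it in place, leaving physics off and the widget hidden.
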(event EventBeginPlay)

(event Collision|EventActorBeginOverlap
  (params (OtherActor :type Actor%20Object%20Reference))
  (if (not (Variables|Default|GetisDone))
    (Default|CallTaskFinish)
    (Variables|Default|SetisDone true)))

(event EventTick
  (params (DeltaSeconds :type Float%20%28single-precision%29)))

(event EventDrop
  (Physics|SetSimulatePhysics (Variables|Default|GetStaticMesh) false)
  (Transformation|DetachFromActor "KeepWorld" "KeepWorld" "KeepWorld"))

(event EventPickup
  (params (AttachTo :type Scene%20Component%20Object%20Reference))
  (Utilities|FlowControl|Sequence
    (:then_1
      (Physics|SetSimulatePhysics (Variables|Default|GetStaticMesh) false)
      (Transformation|AttachComponentToComponent (Variables|Default|GetDefaultSceneRoot) AttachTo "None" "KeepWorld" "KeepWorld" "KeepWorld" false)
      (Rendering|SetVisibility (Variables|Default|GetWidget) false false))))

(fn ConstructionScript)