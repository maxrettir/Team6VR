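; Toothbrush object for Just Focus that BP_MotionController can pick up and drop.
; Pickup turns off mesh physics, attaches the root to the supplied component keeping its world transform, and hides the Widget.
; Drop restores physics and detaches the actor, leaving the Widget hidden.
; SetTarget stores a Target and construction clears IsDone, though neither is used here, and Test2 is a debug print.
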(event EventBeginPlay)

(event Collision|EventActorBeginOverlap
  (params (OtherActor :type Actor%20Object%20Reference)))

(event EventTick
  (params (DeltaSeconds :type Float%20%28single-precision%29)))

(event EventPickup
  (params (AttachTo :type Scene%20Component%20Object%20Reference))
  (Utilities|FlowControl|Sequence
    (:then_0
      (Physics|SetSimulatePhysics (Variables|Debug|GetStaticMeshComponent) false)
      (Transformation|AttachComponentToComponent (VehicleSound|GetRootComponent) AttachTo "None" "KeepWorld" "KeepWorld" "KeepWorld" false)
      (Rendering|SetVisibility (Variables|Default|GetWidget) false true))))

(event EventDrop
  (Utilities|FlowControl|Sequence
    (:then_0
      (Physics|SetSimulatePhysics (Variables|Debug|GetStaticMeshComponent) true)
      (Transformation|DetachFromActor "KeepWorld" "KeepWorld" "KeepWorld"))))

(fn ConstructionScript
  (Variables|Default|SetisDone false))

(fn Test2
  (Development|PrintText "Hello"))

(fn SetTarget
  (params (t :type Plane%20Blueprint%20Object%20Reference))
  (Variables|Default|Settarget t))