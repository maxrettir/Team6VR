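; Plane actor with a text label that tracks a simple task state through an IsDone flag, reset in the construction script.
; Working prints a debug message, uppercases the label and swaps the mesh material to M_HandMat.
; CompleteTask sets the label to the Text variable and sets IsDone.
; The event graph only calls parent BeginPlay; its CompleteTask call is unwired, so both functions rely on outside callers.
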(event EventBeginPlay
  (|CallParentFunction))

(event Collision|EventActorBeginOverlap
  (params (OtherActor :type Actor%20Object%20Reference))
  (|CallParentFunction OtherActor) ; This node is disabled and will not be called.\nDrag off pins to build functionality.
)

(event EventTick
  (params (DeltaSeconds :type Float%20%28single-precision%29))
  (|CallParentFunction DeltaSeconds) ; This node is disabled and will not be called.\nDrag off pins to build functionality.
)

(fn ConstructionScript
  (|CallParentFunction)
  (Variables|Default|SetisDone false))

(fn CompleteTask
  (Rendering|Components|TextRender|SetText (Variables|Default|GetTextRender1) (LocalVariables|Gettext))
  (Variables|Default|SetisDone true))

(fn Working
  (bind _textrender1 (Variables|Default|GetTextRender1))
  (Utilities|FlowControl|Sequence
    (:then_0
      (Development|PrintText "changing" true false))
    (:then_1
      (Rendering|Components|TextRender|SetText _textrender1 (Class|KismetTextLibrary|TexttoUpper (Variables|/Script/Engine.TextRenderComponent|GetText _textrender1))))
    (:then_2
      (Rendering|Material|SetMaterial (Variables|Debug|GetStaticMeshComponent) 0 "/Game/VirtualReality/Mannequin/Character/Materials/M_HandMat.M_HandMat"))))